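; BP_Camino is a three-lane road segment that asks GeneradorCaminos for a new segment when the player overlaps its box, then removes one after a delay.
; BeginPlay records lane transforms and scatters trees, rocks and vegetation on both sides.
; Tick rerolls lane objects, kept by per-tag probability, until EsCaminoValido finds a destroyed entry or one not tagged Frente, aiming to avoid fully blocked roads.
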(event `self.ReceiveBeginPlay`
  (`KismetArrayLibrary.Array_AddUnique` (`self.Carriles`) (`SceneComponent.K2_GetComponentToWorld` (`self.Carril 1`)))
  (`KismetArrayLibrary.Array_AddUnique` (`self.Carriles`) (`SceneComponent.K2_GetComponentToWorld` (`self.Carril 2`)))
  (`KismetArrayLibrary.Array_AddUnique` (`self.Carriles`) (`SceneComponent.K2_GetComponentToWorld` (`self.Carril 3`)))
  (`self.DecoracionProcedural` (`self.AreaArbolesIzquierda`) 5 "/Game/Blueprints/Escenario/Decoracion/BP_Arbol.BP_Arbol_C" 1200.0)
  (`self.DecoracionProcedural` (`self.AreaRocasIzquierda`) 3 "/Game/Blueprints/Escenario/Decoracion/BP_Rocas.BP_Rocas_C" 900.0)
  (`self.DecoracionProcedural` (`self.AreaVegetacionIzquierda`) 5 "/Game/Blueprints/Escenario/Decoracion/BP_Vegetacion.BP_Vegetacion_C" 500.0)
  (`self.DecoracionProcedural` (`self.AreaArbolesDerecha`) 5 "/Game/Blueprints/Escenario/Decoracion/BP_Arbol.BP_Arbol_C" 1200.0)
  (`self.DecoracionProcedural` (`self.AreaRocasDerecha`) 3 "/Game/Blueprints/Escenario/Decoracion/BP_Rocas.BP_Rocas_C" 900.0)
  (`self.DecoracionProcedural` (`self.AreaVegetacionDerecha`) 5 "/Game/Blueprints/Escenario/Decoracion/BP_Vegetacion.BP_Vegetacion_C" 500.0))

(event `self.ReceiveTick`
  (params (DeltaSeconds :type "Float (single-precision)"))
  (bind _esvalido (`self.EsCaminoValido`))
  (if (not _esvalido)
    (for _array_element (`self.ObjetosGenerados`)
      (`self.K2_DestroyActor` _array_element))
    (for _array_element_2 (`self.Carriles`)
      (`self.GenerarObjetos` _array_element_2))))

(event `self.Box.OnComponentBeginOverlap`
  (params (OverlappedComponent :type "PrimitiveComponent Object Reference") (OtherActor :type "Actor Object Reference") (OtherComp :type "PrimitiveComponent Object Reference") (OtherBodyIndex :type Integer) (bFromSweep :type Boolean) (SweepResult :type "HitResult Structure (by ref)"))
  (cast `/Game/Blueprints/Player/BP_Player` OtherActor)
  (bind _returnvalue (`/Game/Blueprints/Escenario/BP_GeneradorMapa.GetTransformUltimoCamino` (`self.GeneradorCaminos`)))
  (`/Game/Blueprints/Escenario/BP_GeneradorMapa.GenerarCamino` (`self.GeneradorCaminos`) _returnvalue)
  (`KismetSystemLibrary.Delay` 2.0)
  (`/Game/Blueprints/Escenario/BP_GeneradorMapa.EliminarCamino` (`self.GeneradorCaminos`)))

(fn `DecoracionProcedural`
  (params (Area :type "BoxComponent Object Reference") (Cantidad :type Integer) (Class :type "Actor Class Reference") (DistanciaAleatoria :type "Float (double-precision)"))
  (bind _returnvalue (`KismetMathLibrary.RandomFloatInRange` (* DistanciaAleatoria -1.0) DistanciaAleatoria))
  (for _ (range (+ Cantidad 1))
    (`|SpawnActorFromClass` Class (`KismetMathLibrary.MakeTransform` (`KismetMathLibrary.MakeVector` (+ (.x (`KismetMathLibrary.RandomPointInBoundingBox` (`SceneComponent.K2_GetComponentLocation` Area) (`BoxComponent.BoxExtent` Area))) _returnvalue) (+ (.y (`KismetMathLibrary.RandomPointInBoundingBox` (`SceneComponent.K2_GetComponentLocation` Area) (`BoxComponent.BoxExtent` Area))) _returnvalue) (.z (`KismetMathLibrary.RandomPointInBoundingBox` (`SceneComponent.K2_GetComponentLocation` Area) (`BoxComponent.BoxExtent` Area))))) "Undefined" "MultiplyWithRoot" null null)))

(fn `EsCaminoValido`
  (returns (Esvalido :type Boolean))
  (if (not (`self.EsValido`))
    (set `self.EsValido` false)
    (for _array_element (`self.ObjetosGenerados`)
      (`/Engine/EditorBlueprintResources/StandardMacros.IsValid` _array_element
        (:`Is Valid`
          (bind _etiqueta (`/Game/Blueprints/Escenario/BP_ObjetosCamino.getTag` _array_element))
          (if (!= _etiqueta (struct :`TagName` "Obstaculo.Frente"))
            (set `self.EsValido` true)))
        (:`Is Not Valid`
          (set `self.EsValido` true))))
    (return (`self.EsValido`))))

(fn `GenerarObjetos`
  (params (InTransform :type "Transform Structure (by ref)"))
  (locals (NewLocalVar :type Boolean))
  (bind _output (`|GetArrayItem` (`self.ObjetosCamino`) (`KismetMathLibrary.RandomIntegerInRange` 0 (- (`KismetArrayLibrary.Array_Length` (`self.ObjetosCamino`)) 1))))
  (if (`KismetSystemLibrary.IsValidClass` _output)
    (bind _returnvalue (`|SpawnActorFromClass` _output (`KismetMathLibrary.MakeTransform` (.location InTransform) (.rotation InTransform)) "Undefined" "MultiplyWithRoot" null null))
    (`/Engine/EditorBlueprintResources/StandardMacros.IsValid` _returnvalue
      (:`Is Valid`
        (bind _etiqueta (`/Game/Blueprints/Escenario/BP_ObjetosCamino.getTag` _returnvalue))
        (if (<= (`KismetMathLibrary.RandomFloatInRange` 0.1 1.0) (`BlueprintMapLibrary.Map_Find` (`self.ProbabilidadAparecer`) _etiqueta))
          (`KismetArrayLibrary.Array_AddUnique` (`self.ObjetosGenerados`) _returnvalue)
          (else
            (`self.K2_DestroyActor` _returnvalue)))))))

(fn `GetCarriles`
  (returns (Carriles :type "Array of Transform Structure"))
  (return (`self.Carriles`)))

(fn `GetObjetosGenerados`
  (returns (ObjetosGenerados :type "Array of /Game/Blueprints/Escenario/BP_ObjetosCamino Object Reference"))
  (return (`self.ObjetosGenerados`)))

(fn `GetPuntoConstruccion`
  (returns (ReturnValue :type "Transform Structure"))
  (return (`SceneComponent.K2_GetComponentToWorld` (`self.PuntoConstruccion`))))

(fn `SetGeneradorCaminos`
  (params (GeneradorCaminos :type "/Game/Blueprints/Escenario/BP_GeneradorMapa Object Reference"))
  (set `self.GeneradorCaminos` GeneradorCaminos))

(fn `UserConstructionScript`)