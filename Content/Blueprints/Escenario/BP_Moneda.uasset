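; BP_Moneda is a coin pickup that the player collects on collision.
; It overrides an inherited Collision function: after the parent call, it casts to BP_Player, calls Recoger, plays a sound, spawns a fire particle effect and hides its mesh.
; A Destructor event then waits briefly before destroying the actor and the spawned particle component.
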(event `Destructor`
  (`KismetSystemLibrary.Delay` 2.0)
  (`self.K2_DestroyActor`)
  (`ActorComponent.K2_DestroyComponent` (`self.Particulas`)))

(fn `Collision`
  (params (NewParam :type "Actor Object Reference"))
  (bind _returnvalue (`self.K2_GetActorLocation`))
  (`parent.Collision` NewParam)
  (bind _asbp_player (cast `/Game/Blueprints/Player/BP_Player` NewParam))
  (`/Game/Blueprints/Player/BP_Player.Recoger` _asbp_player)
  (`GameplayStatics.PlaySoundAtLocation` "/Engine/VREditor/Sounds/UI/Leave_Simulate.Leave_Simulate" _returnvalue (struct) 1.0 1.0 0.0 null null null null)
  (bind _returnvalue_2 (`GameplayStatics.SpawnEmitterAtLocation` "/Game/PlantillasUE5/StarterContent/Particles/P_Fire.P_Fire" _returnvalue (struct :`Pitch` 90.0) (2.0 2.0 2.0)))
  (set `self.Particulas` _returnvalue_2)
  (`SceneComponent.SetVisibility` (`self.StaticMesh`) false false)
  (`self.Destructor`))

(fn `UserConstructionScript`
  (`parent.UserConstructionScript`))