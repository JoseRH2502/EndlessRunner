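; Map generator for an endless runner that chains random path segments and raises difficulty as the player travels.
; BeginPlay spawns the initial segments end to end, each receiving the current spawn probabilities, then copies the second segment's lane positions to BP_Player.
; EliminarCamino removes the oldest segment with its spawned objects.
; Tick checks player distance, periodically adding per-tag increments to coin and obstacle probabilities and increasing player speed.
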(event `self.ReceiveBeginPlay`
  (`|ExecutionSequence`
    (:`then_0`
      (for _index (range (+ (`self.NumCaminosInciales`) 1))
        (if (== _index 0)
          (`self.GenerarCamino` (`self.GetTransform`))
          (else
            (`self.GenerarCamino` (`/Game/Blueprints/Escenario/BP_Camino.GetPuntoConstruccion` (`|GetArrayItem` (`self.Caminos`) (- _index 1))))))))
    (:`then_1`
      (`self.ConfiguracionCarriles`))
    (:`then_2`
      (bind _asbp_player (cast `/Game/Blueprints/Player/BP_Player` (`GameplayStatics.GetPlayerPawn` 0)))
      (set `self.BP Player` _asbp_player)
      (set `self.SiguienteDistanciaParaAumentarDificultad` (`self.DistanciaParaAumentarDificultad`)))))

(event `self.ReceiveTick`
  (params (DeltaSeconds :type "Float (single-precision)"))
  (`self.AumentarDificultad`))

(fn `AumentarDificultad`
  (locals (TempProbabilidades :type "Map of GameplayTag Structure to Float (double-precision)"))
  (bind _returnvalue (`BlueprintGameplayTagLibrary.MakeLiteralGameplayTag` (struct :`TagName` "Obstaculo.Abajo")))
  (bind _returnvalue_2 (`BlueprintGameplayTagLibrary.MakeLiteralGameplayTag` (struct :`TagName` "Obstaculo.Arriba")))
  (bind _returnvalue_3 (`BlueprintGameplayTagLibrary.MakeLiteralGameplayTag` (struct :`TagName` "Obstaculo.Frente")))
  (bind _returnvalue_4 (`BlueprintGameplayTagLibrary.MakeLiteralGameplayTag` (struct :`TagName` "Moneda")))
  (if (> (`/Game/Blueprints/Player/BP_Player.GetDistancia` (`self.BP Player`)) (`self.SiguienteDistanciaParaAumentarDificultad`))
    (`|ExecutionSequence`
      (:`then_0`
        (bind _returnvalue_5 (`self.CalcularEscalado` _returnvalue_4))
        (`BlueprintMapLibrary.Map_Add` (`local.TempProbabilidades`) _returnvalue_4 _returnvalue_5))
      (:`then_1`
        (bind _returnvalue_6 (`self.CalcularEscalado` _returnvalue))
        (`BlueprintMapLibrary.Map_Add` (`local.TempProbabilidades`) _returnvalue _returnvalue_6))
      (:`then_2`
        (bind _returnvalue_7 (`self.CalcularEscalado` _returnvalue_2))
        (`BlueprintMapLibrary.Map_Add` (`local.TempProbabilidades`) _returnvalue_2 _returnvalue_7))
      (:`then_3`
        (bind _returnvalue_8 (`self.CalcularEscalado` _returnvalue_3))
        (`BlueprintMapLibrary.Map_Add` (`local.TempProbabilidades`) _returnvalue_3 _returnvalue_8))
      (:`then_4`
        (set `self.Probabilidades` (`local.TempProbabilidades`))
        (set `self.SiguienteDistanciaParaAumentarDificultad` (+ (`self.SiguienteDistanciaParaAumentarDificultad`) (`self.DistanciaParaAumentarDificultad`)))
        (`/Game/Blueprints/Player/BP_Player.AumentarValocidad` (`self.BP Player`))))))

(fn `CalcularEscalado`
  (params (Etiqueta :type "GameplayTag Structure (by ref)"))
  (returns (ReturnValue :type "Float (double-precision)"))
  (return (+ (`BlueprintMapLibrary.Map_Find` (`self.EscaladoProbabilidades`) Etiqueta) (`BlueprintMapLibrary.Map_Find` (`self.Probabilidades`) Etiqueta))))

(fn `ConfiguracionCarriles`
  (locals (LocalPlayer :type "/Game/Blueprints/Player/BP_Player Object Reference"))
  (bind _asbp_player (cast `/Game/Blueprints/Player/BP_Player` (`GameplayStatics.GetPlayerPawn` 0)))
  (set `local.LocalPlayer` _asbp_player)
  (`KismetArrayLibrary.Array_Clear` (`/Game/Blueprints/Player/BP_Player.Carriles` (`local.LocalPlayer`)))
  (bind _carriles (`/Game/Blueprints/Escenario/BP_Camino.GetCarriles` (`|GetArrayItem` (`self.Caminos`) 1)))
  (for _array_element _carriles
    (`KismetArrayLibrary.Array_Add` (`/Game/Blueprints/Player/BP_Player.Carriles` (`local.LocalPlayer`)) (.y (.location _array_element)))))

(fn `EliminarCamino`
  (locals (CaminoAEliminar :type "/Game/Blueprints/Escenario/BP_Camino Object Reference"))
  (set `local.CaminoAEliminar` (`|GetArrayItem` (`self.Caminos`)))
  (`KismetArrayLibrary.Array_RemoveItem` (`self.Caminos`) (`local.CaminoAEliminar`))
  (for _array_element (`/Game/Blueprints/Escenario/BP_Camino.GetObjetosGenerados` (`local.CaminoAEliminar`))
    (`/Engine/EditorBlueprintResources/StandardMacros.IsValid` _array_element
      (:`Is Valid`
        (`self.K2_DestroyActor` _array_element)
        (`self.ConfiguracionCarriles`))))
  (`self.K2_DestroyActor` (`local.CaminoAEliminar`)))

(fn `GenerarCamino`
  (params (SpawnTransform :type "Transform Structure"))
  (bind _returnvalue (`|SpawnActorFromClass` (`|GetArrayItem` (`self.ClasesCaminos`) (`KismetMathLibrary.RandomIntegerInRange` 0 (- (`KismetArrayLibrary.Array_Length` (`self.ClasesCaminos`)) 1))) SpawnTransform "Undefined" "MultiplyWithRoot" null (`self.Probabilidades`) null))
  (`/Game/Blueprints/Escenario/BP_Camino.SetGeneradorCaminos` _returnvalue self)
  (`KismetArrayLibrary.Array_AddUnique` (`self.Caminos`) _returnvalue))

(fn `GetTransformUltimoCamino`
  (returns (ReturnValue :type "Transform Structure (by ref)"))
  (return (`/Game/Blueprints/Escenario/BP_Camino.GetPuntoConstruccion` (`|GetArrayItem` (`self.Caminos`) (- (`KismetArrayLibrary.Array_Length` (`self.Caminos`)) 1)))))

(fn `UserConstructionScript`)