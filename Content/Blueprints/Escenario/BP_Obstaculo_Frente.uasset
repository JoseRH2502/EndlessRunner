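; BP_Obstaculo_Frente is a scenery obstacle actor that varies its appearance each time it spawns.
; On BeginPlay it sets a random yaw over a full turn and assigns its StaticMesh component a random entry from the Mesh array.
; The construction script only calls its parent, so the variation appears at runtime; overlap and tick events are disabled.
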(event `self.ReceiveBeginPlay`
  (`parent.ReceiveBeginPlay`)
  (`self.K2_SetActorRotation` (`KismetMathLibrary.MakeRotator` 0.0 0.0 (`KismetMathLibrary.RandomFloatInRange` 0.0 360.0)))
  (`StaticMeshComponent.SetStaticMesh` (`self.StaticMesh`) (`|GetArrayItem` (`self.Mesh`) (`KismetMathLibrary.RandomIntegerInRange` 0 (- (`KismetArrayLibrary.Array_Length` (`self.Mesh`)) 1)))))

(fn `UserConstructionScript`
  (`parent.UserConstructionScript`))